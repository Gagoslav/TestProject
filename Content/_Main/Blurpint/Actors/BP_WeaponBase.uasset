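; Base weapon actor that can be attached to a character mesh and fired as a hitscan gun through interfaces.
; Attaching snaps it to its configured socket and returns its weapon type.
; Firing traces from screen center against Pawn objects, plays sound and a muzzle-socket emitter, and returns the hit without applying damage.
; MakeUnequipedFor temporarily clears CanBeEquipped, restoring it after a delay.
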(event `MakeUnequipedFor`
  (params (InSecs :type "Float (double-precision)"))
  (set `self.CanBeEquipped` false)
  (`KismetSystemLibrary.Delay` InSecs)
  (set `self.CanBeEquipped` true))

(fn `Custom Function`)

(fn `I_WeaponAttache`
  (params (SkelitalMesh :type "SceneComponent Object Reference"))
  (returns (Weapontype :type "/Game/_Main/Blurpint/Data/E_WeaponType Enum"))
  (`self.K2_AttachToComponent` SkelitalMesh (`self.WeaponSocketName`) "SnapToTarget" "SnapToTarget" "SnapToTarget")
  (return (`self.Enum_WeaponType`)))

(fn `I_WeaponFire`
  (params (NewParam1 :type "Pawn Object Reference") (Skelitolmesh :type "Character Object Reference"))
  (returns (NewParam :type "HitResult Structure"))
  (bind (_returnvalue_location _returnvalue_rotation _returnvalue_scale) (`KismetMathLibrary.BreakTransform` (`SceneComponent.GetSocketTransform` (`self.SM_Weapon`) (`self.MuzleFlasSocket Name`) "RTS_World")))
  (bind (_worldposition _worlddirection) (`GameplayStatics.DeprojectScreenToWorld` (`GameplayStatics.GetPlayerController` 0) (/ (`WidgetLayoutLibrary.GetViewportSize`) (2.0 2.0))))
  (bind _outhit (`KismetSystemLibrary.LineTraceSingleForObjects` _worldposition (+ _worldposition (* _worlddirection 5000.0)) (`|MakeArray` "ObjectTypeQuery3" :!type "EObjectTypeQuery Enum") true (`|MakeArray` NewParam1 :!type "Actor Object Reference")))
  (`GameplayStatics.PlaySound2D` (`self.WeaponSound`) 0.05 1.0 0.0 null null)
  (`GameplayStatics.SpawnEmitterAtLocation` (`self.WeaponEmitter`) _returnvalue_location _returnvalue_rotation _returnvalue_scale)
  (return _outhit))

(fn `UserConstructionScript`)