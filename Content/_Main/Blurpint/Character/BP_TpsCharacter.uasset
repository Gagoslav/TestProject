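; Multiplayer third-person shooter character that picks up, drops, aims, fires and reloads rifles or pistols.
; Actions route through Server_ events to Client_ or Multi_ events, calling weapons through interfaces and updating montages, pose state, ammo and HUD.
; Hit actors receive a health message that removes fixed damage, plays a reaction and, at zero, triggers ragdoll and a retry menu.
; Control pitch is relayed similarly, and sprinting lerps spring-arm length by timeline.
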(event `Server_Fire`
  (bind _attachweaponref (`self.AttachWeaponRef`))
  ;[0.4597 0.4957 1] WeaponFire
  (if (and (not (== (`self.CurentAmo`) 0)) (not (`self.bIsReload?`)))
    (`/Engine/EditorBlueprintResources/StandardMacros.IsValid` _attachweaponref
      (:`Is Valid`
        (bind _newparam (message `/Game/_Main/Blurpint/Interface/BPI_WeaponIntraction.I_WeaponFire` _attachweaponref self self))
        (`|ExecutionSequence`
          (:`then_0`
            (set `self.CurentAmo` (`KismetMathLibrary.Clamp` (- (`self.CurentAmo`) 1) 0 30)))
          (:`then_1`
            (bind (_bblockinghit _binitialoverlap _time _distance _location _impactpoint _normal _impactnormal _physmat _hitactor) (`GameplayStatics.BreakHitResult` _newparam))
            (`self._Heal` _hitactor))
          (:`then_2`
            (`self.Server_ShootAnim`))
          (:`then_3`
            (if _bblockinghit
              _)))))))

(event `_Heal`
  (params (Target :type "Object Object Reference"))
  ;[0.4597 0.4957 1] WeaponFire
  (message `/Game/_Main/Blurpint/Interface/BPI_FpsCharacter.HealthUpda` Target 0.0))

(event `Client_UnequipWeapon`
  (bind _wbp_mainhudref (`self.WBP_MainHudRef`))
  (bind _attachweaponref (`self.AttachWeaponRef`))
  ;[0.4597 0.4957 1] Weapon Equiped and Unequiped
  (`/Engine/EditorBlueprintResources/StandardMacros.IsValid` _attachweaponref
    (:`Is Valid`
      (`/Game/_Main/Blurpint/Actors/BP_WeaponBase.MakeUnequipedFor` _attachweaponref 1.0)
      (`self.K2_DetachFromActor` _attachweaponref "KeepRelative" "KeepRelative" "KeepRelative")
      (`self.K2_SetActorLocation` _attachweaponref (+ (`self.K2_GetActorLocation`) (+ (`KismetMathLibrary.GetForwardVector` (`self.K2_GetActorRotation`)) (250.0 0.0 0.0))) false false)
      (set `self.AttachWeaponRef` null)
      (set `self.EnumPlayerState` (select `/Game/_Main/Blurpint/Data/E_WeaponType` (`self.Weapontype`) :`NewEnumerator0` "NewEnumerator0" :`NewEnumerator1` "NewEnumerator0" :`NewEnumerator2` "NewEnumerator0" :!type "/Game/_Main/Blurpint/Data/E_PlayerState Enum"))
      (`/Engine/EditorBlueprintResources/StandardMacros.IsValid` _wbp_mainhudref
        (:`Is Valid`
          (`/Game/_Main/UI/WBP_MainHud._UpdateWeaponSlot` _wbp_mainhudref null))))))

(event `self.ReceiveBeginPlay`
  ;[0 1 0.8715] Begin Play logic
  (set `self.DefaultArmLength` (`SpringArmComponent.TargetArmLength` (`self.SpringArm`)))
  (`KismetSystemLibrary.DelayUntilNextTick`)
  (if (`self.IsLocallyControlled`)
    (bind _returnvalue (`|CreateWidget` "/Game/_Main/UI/WBP_MainHud.WBP_MainHud_C"))
    (bind _output_get (set `self.WBP_MainHudRef` _returnvalue))
    (`/Engine/EditorBlueprintResources/StandardMacros.IsValid` _output_get
      (:`Is Valid`
        (`UserWidget.AddToViewport` _output_get 0)))))

(event `server_UnequipeWeapon`
  ;[0.4597 0.4957 1] Weapon Equiped and Unequiped
  (`self.Client_UnequipWeapon`))

(event `Server_ShootAnim`
  ;[0.4597 0.4957 1] WeaponFire
  (`self.Cleint_ShootAnim`))

(event `Cleint_ShootAnim`
  ;[0.4597 0.4957 1] WeaponFire
  (`self.PlayAnimMontage` (select `/Game/_Main/Blurpint/Data/E_WeaponType` (`self.Weapontype`) :`NewEnumerator1` "/Game/AnimStarterPack/Montages/Fire_Rifle_Ironsights_Montage.Fire_Rifle_Ironsights_Montage" :`NewEnumerator2` "/Game/AnimStarterPack/Montages/AM_Idle_Pistol_Fire.AM_Idle_Pistol_Fire" :!type "AnimMontage Object Reference")))

(event `Server_Pitch`
  (params (PitchRotate :type "Float (double-precision)"))
  ;[0 1 0.8715] Begin Play logic
  (`self.Client_Pitch` PitchRotate))

(event `Key|E`
  (params (Key :type "Key Structure"))
  ;[0.4597 0.4957 1] Weapon Equiped and Unequiped
  (:`Pressed`
    (`self.server_UnequipeWeapon`)))

(event `Key|LeftMouseButton`
  (params (Key :type "Key Structure"))
  ;[0.4597 0.4957 1] WeaponFire
  (:`Pressed`
    (if (not (`self.IsSprinting`))
      (`self.Server_Fire`))))

(event `UnEquipWeapon`
  ;[0.4597 0.4957 1] Weapon Equiped and Unequiped
)

(event `Client_Pitch`
  (params (PitchRotate :type "Float (double-precision)"))
  ;[0 1 0.8715] Begin Play logic
  (set `self.PitchRotate` PitchRotate))

(event `InputAxisKey|MouseX`
  (params (AxisValue :type "Float (single-precision)"))
  ;[0 1 0.8715] Begin Play logic
  (`self.AddControllerYawInput` AxisValue))

(event `Key|One`
  (params (Key :type "Key Structure"))
  ;[0.4597 0.4957 1] WeaponFire
)

(event `Server_WeaponEquped`
  (params (AttachWeaponRef :type "/Game/_Main/Blurpint/Actors/BP_WeaponBase Object Reference"))
  ;[0.4597 0.4957 1] Weapon Equiped and Unequiped
  (`self.Client_WeaponEquped` AttachWeaponRef))

(event `InputAxisKey|MouseY`
  (params (AxisValue :type "Float (single-precision)"))
  (bind (_returnvalue_roll _returnvalue_pitch) (`KismetMathLibrary.BreakRotator` (`self.GetControlRotation`)))
  ;[0 1 0.8715] Begin Play logic
  (`self.AddControllerPitchInput` AxisValue)
  (`self.Server_Pitch` _returnvalue_pitch))

(event `self.OnJumped`
  ;[0 1 0.8715] Begin Play logic
  (if (`self.bIsCrouched`)
    (`self.UnCrouch`)))

(event `Server_UpdateWeaponslot`
  ;[0.4597 0.4957 1] Weapon Equiped and Unequiped
  (`self.Client_UpdateWeaponslot`))

(event `Client_WeaponEquped`
  (params (AttachWeaponRef :type "/Game/_Main/Blurpint/Actors/BP_WeaponBase Object Reference"))
  ;[0.4597 0.4957 1] Weapon Equiped and Unequiped
  (bind _output_get (set `self.AttachWeaponRef` AttachWeaponRef))
  (`/Engine/EditorBlueprintResources/StandardMacros.IsValid` _output_get
    (:`Is Valid`
      (bind _weapontype (message `/Game/_Main/Blurpint/Interface/BPI_WeaponIntraction.I_WeaponAttache` _output_get (`self.Mesh`)))
      (set `self.Weapontype` _weapontype)
      (`self.SetOwner` _output_get self))))

(event `Server_health`
  ;[0.4597 0.4957 1] PlayerHealth
  (`|ExecutionSequence`
    (:`then_0`
      (bind _output_get (set `self.Health` (`KismetMathLibrary.FClamp` (- (`self.Health`) 0.1))))
      (if (== _output_get 0.0)
        (`self.Server_Rogdoll`)))
    (:`then_1`
      (`self.Server_Hireaction`))))

(event `/Game/_Main/Blurpint/Interface/BPI_FpsCharacter.HealthUpda`
  (params (NewParam :type "Float (double-precision)"))
  ;[0.4597 0.4957 1] PlayerHealth
  (`self.Server_health`))

(event `Key|RightMouseButton`
  (params (Key :type "Key Structure"))
  ;[0.4597 0.4957 1] Weapon Equiped and Unequiped
  (:`Pressed`
    (if (not (`self.IsSprinting`))
      (`self.Server_WeaponAim`)))
  (:`Released`
    (`self.Server_WeaponaimRelease`)))

(event `Client_UpdateWeaponslot`
  (bind _weapontype (`self.Weapontype`))
  (bind _wbp_mainhudref (`self.WBP_MainHudRef`))
  ;[0.4597 0.4957 1] Weapon Equiped and Unequiped
  (set `self.EnumPlayerState` (select `/Game/_Main/Blurpint/Data/E_WeaponType` _weapontype :`NewEnumerator0` "NewEnumerator0" :`NewEnumerator1` "NewEnumerator6" :`NewEnumerator2` "NewEnumerator7" :!type "/Game/_Main/Blurpint/Data/E_PlayerState Enum"))
  (`/Engine/EditorBlueprintResources/StandardMacros.IsValid` _wbp_mainhudref
    (:`Is Valid`
      (`/Game/_Main/UI/WBP_MainHud._UpdateWeaponSlot` _wbp_mainhudref (select `/Game/_Main/Blurpint/Data/E_WeaponType` _weapontype :`NewEnumerator1` (`self.WeaponRifleIcon`) :`NewEnumerator2` (`self.WeaponPistolIcon`) :!type "Object Object Reference"))
      (set `self.TotalAmo` (select `/Game/_Main/Blurpint/Data/E_WeaponType` (`self.Weapontype`) :`NewEnumerator1` 120 :`NewEnumerator2` 25))
      (set `self.CurentAmo` (select `/Game/_Main/Blurpint/Data/E_WeaponType` (`self.Weapontype`) :`NewEnumerator1` 30 :`NewEnumerator2` 7)))))

(event `Server_Hireaction`
  ;[0.4597 0.4957 1] PlayerHealth
  (`self.Client_HitReaction`))

(event `Client_HitReaction`
  ;[0.4597 0.4957 1] PlayerHealth
  (`self.PlayAnimMontage` "/Game/AnimStarterPack/Montages/AM_Hit_React_2.AM_Hit_React_2"))

(event `Server_Rogdoll`
  ;[0.4597 0.4957 1] PlayerHealth
  (`self.Multi_Rogdoll`))

(event `Multi_Rogdoll`
  ;[0.4597 0.4957 1] PlayerHealth
  (`PrimitiveComponent.SetSimulatePhysics` (`self.Mesh`) true)
  (`self._Retry`))

(event `self.OnStartSprint`
  ;[1 1 1] Make camera move back on start sprint
  (set `self.IsSprinting` true)
  (set `self.bUseControllerRotationYaw` false)
  (bind (_direction _alpha) (`Timeline|SpringArmTimeline` :!label _label)
    (:`Update`
      (set `SpringArmComponent.TargetArmLength` (`KismetMathLibrary.Lerp` (`self.DefaultArmLength`) (`self.NewTargetLength`) _alpha) (`self.SpringArm`)))))

(event `_Retry`
  ;[0.4597 0.4957 1] PlayerHealth
  (if (`self.IsLocallyControlled`)
    (`KismetSystemLibrary.Delay` 1.0)
    (bind _returnvalue (`|CreateWidget` "/Game/_Main/UI/WBP_RetraiManu.WBP_RetraiManu_C"))
    (`UserWidget.AddToViewport` _returnvalue 0)
    (`self._ShowMouse`)))

(event `self.OnEndSprint`
  ;[1 1 1] Make camera move back on start sprint
  (set `self.IsSprinting` false)
  (set `self.bUseControllerRotationYaw` true)
  (goto _label :!via `Reverse`))

(event `_ShowMouse`
  (bind _returnvalue (`GameplayStatics.GetPlayerController` 0))
  ;[0.4597 0.4957 1] PlayerHealth
  (set `PlayerController.bShowMouseCursor` true _returnvalue)
  (`WidgetBlueprintLibrary.SetInputMode_UIOnlyEx` _returnvalue (stale `_Retry` _returnvalue)))

(event `self.CapsuleComponent.OnComponentHit`
  (params (HitComponent :type "PrimitiveComponent Object Reference") (OtherActor :type "Actor Object Reference") (OtherComp :type "PrimitiveComponent Object Reference") (NormalImpulse :type "Vector Structure") (Hit :type "HitResult Structure (by ref)"))
  (if (`self.IsSprinting`)
    (`self.EndSprint`)))

(event `InputAction|Reload`
  (params (Key :type "Key Structure"))
  ;[0.4597 0.4957 1] Weapon Reload
  (:`Pressed`
    (`/Engine/EditorBlueprintResources/StandardMacros.DoOnce` false :!label _label_2
      (:`Completed`
        (if (and (not (== (`self.CurentAmo`) (select `/Game/_Main/Blurpint/Data/E_WeaponType` (`self.Weapontype`) :`NewEnumerator1` 30 :`NewEnumerator2` 7))) (not (== (`self.TotalAmo`) 0)))
          (set `self.bIsReload?` true)
          (`self.Server_Reload`))))))

(event `Server_WeaponAim`
  ;[0.4597 0.4957 1] Weapon Equiped and Unequiped
  (`self.Client_WeaponAim`))

(event `Server_Reload`
  ;[0.4597 0.4957 1] Weapon Reload
  (`self.Client_Reload`))

(event `Client_WeaponAim`
  (bind _wbp_mainhudref (`self.WBP_MainHudRef`))
  (bind _attachweaponref (`self.AttachWeaponRef`))
  ;[0.4597 0.4957 1] Weapon Equiped and Unequiped
  (`/Engine/EditorBlueprintResources/StandardMacros.IsValid` _attachweaponref
    (:`Is Valid`
      (message `/Game/_Main/Blurpint/Interface/BPI_WeaponIntraction.I_WeaponAim` _attachweaponref (`self.CameraComponent`))
      (`/Engine/EditorBlueprintResources/StandardMacros.IsValid` _wbp_mainhudref
        (:`Is Valid`
          (`/Game/_Main/UI/WBP_MainHud.ShowCroshHair` _wbp_mainhudref "Visible")
          (set `self.EnumPlayerState` (select `/Game/_Main/Blurpint/Data/E_WeaponType` (`self.Weapontype`) :`NewEnumerator0` "NewEnumerator0" :`NewEnumerator1` "NewEnumerator2" :`NewEnumerator2` "NewEnumerator4" :!type "/Game/_Main/Blurpint/Data/E_PlayerState Enum")))))))

(event `Client_Reload`
  (bind _returnvalue (select `/Game/_Main/Blurpint/Data/E_WeaponType` (`self.Weapontype`) :`NewEnumerator1` "/Game/AnimStarterPack/Montages/AM_RifleReload.AM_RifleReload" :`NewEnumerator2` "/Game/AnimStarterPack/Montages/AM_PistolReload.AM_PistolReload" :!type "AnimMontage Object Reference"))
  ;[0.4597 0.4957 1] Weapon Reload
  (`/Engine/EditorBlueprintResources/StandardMacros.IsValid` _returnvalue
    (:`Is Valid`
      (`|PlayMontage` (`self.Mesh`) _returnvalue
        (:`OnCompleted`
          (`self.Server_ReloadAmo`)
          (goto _label_2 :!via `Reset`))))))

(event `Server_WeaponaimRelease`
  ;[0.4597 0.4957 1] Weapon Equiped and Unequiped
  (`self.Client_WeaponaimRelease`))

(event `Client_WeaponaimRelease`
  ;[0.4597 0.4957 1] Weapon Equiped and Unequiped
  (`SceneComponent.K2_SetRelativeLocation` (`self.CameraComponent`) (0.0 0.0 0.0) false false)
  (set `self.EnumPlayerState` (select `/Game/_Main/Blurpint/Data/E_WeaponType` (`self.Weapontype`) :`NewEnumerator0` "NewEnumerator0" :`NewEnumerator1` "NewEnumerator6" :`NewEnumerator2` "NewEnumerator7" :!type "/Game/_Main/Blurpint/Data/E_PlayerState Enum")))

(event `Server_ReloadAmo`
  ;[0.4597 0.4957 1] Weapon Reload
  (`self.Client_ReloadAmo`))

(event `Client_ReloadAmo`
  (bind _returnvalue (- (select `/Game/_Main/Blurpint/Data/E_WeaponType` (`self.Weapontype`) :`NewEnumerator1` 30 :`NewEnumerator2` 7) (`self.CurentAmo`)))
  ;[0.4597 0.4957 1] Weapon Reload
  (set `self.TotalAmo` (`KismetMathLibrary.Clamp` (- (`self.TotalAmo`) _returnvalue) 0 200))
  (set `self.CurentAmo` (+ (`self.CurentAmo`) _returnvalue))
  (set `self.bIsReload?` false))

(event `self.CapsuleComponent.OnComponentBeginOverlap`
  (params (OverlappedComponent :type "PrimitiveComponent Object Reference") (OtherActor :type "Actor Object Reference") (OtherComp :type "PrimitiveComponent Object Reference") (OtherBodyIndex :type Integer) (bFromSweep :type Boolean) (SweepResult :type "HitResult Structure (by ref)"))
  (if (`KismetMathLibrary.ClassIsChildOf` (`GameplayStatics.GetObjectClass` OtherActor) "/Game/_Main/Blurpint/Actors/BP_WeaponBase.BP_WeaponBase_C")
    (bind _asbp_weapon_base (cast `/Game/_Main/Blurpint/Actors/BP_WeaponBase` OtherActor))
    (if (`/Game/_Main/Blurpint/Actors/BP_WeaponBase.CanBeEquipped` _asbp_weapon_base)
      (`|ExecutionSequence`
        (:`then_0`
          (`self.Server_WeaponEquped` _asbp_weapon_base))
        (:`then_1`
          (`self.Server_UpdateWeaponslot`))))))

(fn `UserConstructionScript`)