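; GM_TpsPrototype is a third-person shooter prototype game mode that spawns players at random Player Starts.
; SpawnPlayer destroys the controller's existing pawn, spawns a BP_TpsCharacter at the transform from PlayerStartLocation, and possesses it.
; PlayerStartLocation picks from all PlayerStart actors, re-rolling the random index on each read, so the validated start can differ from the returned one.
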(event `self.ReceiveBeginPlay`)

(event `SpawnPlayer`
  (params (PlayerControl :type "PlayerController Object Reference"))
  (bind _returnvalue (`Controller.K2_GetPawn` PlayerControl))
  (`/Engine/EditorBlueprintResources/StandardMacros.IsValid` _returnvalue
    (:`Is Valid`
      (`self.K2_DestroyActor` _returnvalue))
    (:`Is Not Valid`
      _))
  (bind _returnvalue_2 (`|SpawnActorFromClass` "/Game/_Main/Blurpint/Character/BP_TpsCharacter.BP_TpsCharacter_C" (`self.PlayerStartLocation`) "Undefined" "MultiplyWithRoot" null (0.0 45.0 45.0) (210.0 60.0 60.0) null))
  (`Controller.Possess` PlayerControl _returnvalue_2))

(fn `PlayerStartLocation`
  (returns (Output_Get :type "Transform Structure"))
  (bind _outactors (`GameplayStatics.GetAllActorsOfClass` "/Script/Engine.PlayerStart"))
  (bind _output (`|GetArrayItem` _outactors (`KismetMathLibrary.RandomIntegerInRange` 0 (- (`KismetArrayLibrary.Array_Length` _outactors) 1))))
  (bind _output_get (set `self.PlayerStartRef` _output))
  (`/Engine/EditorBlueprintResources/StandardMacros.IsValid` _output_get
    (:`Is Valid`
      (bind _returnvalue (`self.GetTransform` _output))
      (set `self.PlayerStartTransform` _returnvalue)
      (return _returnvalue))))

(fn `UserConstructionScript`)